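; Projectile actor that flies along the world X axis and rewards the player for hitting health packs or enemies.
; It moves by a swept offset each tick at its forward speed and expires after a short lifespan.
; Sphere overlaps ignore the player; a health pack adds capped health and is destroyed, while an enemy adds score without itself being destroyed here.
; The projectile destroys itself after either hit.
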(event `self.ReceiveBeginPlay`
  (`self.SetLifeSpan` 3.0))

(event `self.ReceiveTick`
  (params (DeltaSeconds :type "Float (single-precision)"))
  (`self.K2_AddActorWorldOffset` (`KismetMathLibrary.MakeVector` (* DeltaSeconds (`self.ForwardSpeed`))) true))

(event `self.Sphere.OnComponentBeginOverlap`
  (params (OverlappedComponent :type "PrimitiveComponent Object Reference") (OtherActor :type "Actor Object Reference") (OtherComp :type "PrimitiveComponent Object Reference") (OtherBodyIndex :type Integer) (bFromSweep :type Boolean) (SweepResult :type "HitResult Structure (by ref)"))
  (bind _player (`self.Player`))
  (bind _player_2 (`self.Player`))
  (cast `/Game/InfiniteMatrix/Blueprints/BP_Player` OtherActor
    (:`CastFailed`
      (bind _ashealth_pack (cast `/Game/InfiniteMatrix/Blueprints/HealthPack` OtherActor)
        (:`then`
          (set `/Game/InfiniteMatrix/Blueprints/BP_Player.CurrHealth` (`KismetMathLibrary.Min` 100 (+ (`/Game/InfiniteMatrix/Blueprints/BP_Player.CurrHealth` _player) 25)) _player)
          (`self.K2_DestroyActor` _ashealth_pack))
        (:`CastFailed`
          (cast `/Game/InfiniteMatrix/Blueprints/Enemy` OtherActor)
          (set `/Game/InfiniteMatrix/Blueprints/BP_Player.Score` (+ (`/Game/InfiniteMatrix/Blueprints/BP_Player.Score` _player_2) 25) _player_2)))
      (`self.K2_DestroyActor`))))

(fn `UserConstructionScript`)